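; Counter switch that, on each PressF event, advances a single-digit count shown on a text render and toggles linked actors between play and stop.
; The count increments, wraps to zero after nine, then updates the display.
; Its parity then drives the Actors array through the BPI_PlayStop interface, calling DoPlayAndStop with true for odd counts and false for even ones.
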(event EventPressF
  (Utilities|FlowControl|Sequence
    (:then_0
      ;[0.15 0.15 0.15 0.5] 카운트 증가 표시
      (CallFunction|카운트증가표시))
    (:then_1
      (if (== (Math|Integer|%(Integer) (Variables|Default|Getcounter) 2) 1)
        (CallFunction|움직이는것)
        (else
          (CallFunction|멈추는것))))))

(fn ConstructionScript)

(fn 움직이는것
  (for _array_element (Variables|Default|Getactors)
    (bind _asbpi_play_stop (Utilities|Casting|CastToBPI_PlayStop _array_element))
    (Default|DoPlayandStop _asbpi_play_stop true)))

(fn 멈추는것
  (for _array_element (Variables|Default|Getactors)
    (bind _asbpi_play_stop (Utilities|Casting|CastToBPI_PlayStop _array_element))
    (Default|DoPlayandStop _asbpi_play_stop false)))

(fn 카운트증가표시
  (CallFunction|Countup)
  (CallFunction|Over9count0)
  (CallFunction|Showcount))

(fn Countup
  ;[0.15 0.15 0.15 0.5] count를 1씩 증가
  (Variables|Default|Setcounter (+ (Variables|Default|Getcounter) 1)))

(fn Over9count0
  ;[0.15 0.15 0.15 0.5] count가  9보다 크면
  (if (> (Variables|Default|Getcounter) 9)
    ;[0.15 0.15 0.15 0.5] count 0으로 변경
    (Variables|Default|Setcounter 0)))

(fn Showcount
  ;[0.15 0.15 0.15 0.5] count를 text render에 표시
  (Rendering|Components|TextRender|SetText (Variables|Default|GetTextRender) (Utilities|Text|ToText(Integer) (Variables|Default|Getcounter))))