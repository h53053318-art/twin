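; BP_LEFTRIGHT is a switch-controlled moving actor whose Box slides back and forth along its relative X axis.
; On BeginPlay it binds to the Switch's update dispatcher, and EventSwitchToggle and DoPlayAndStop provide ways to set the Isplay flag.
; While Isplay is true, Tick moves the Box a fixed step per frame, independent of delta time, and flips direction at either travel limit.
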(event EventBeginPlay
  (EventDispatchers|BindEventtoEventDispatcherUpdateSwitch (Variables|Default|GetSwitch) (EventDispatchers|CreateEvent :!event EventSwitchToggle)))

(event EventTick
  (params (DeltaSeconds :type Float%20%28single-precision%29))
  (if (Variables|Default|Getisplay)
    (if (Variables|Default|Get오른쪽%20%20이동인가?)
      (CallFunction|오른쪽으로이동)
      (if (>= (Variables|Default|GetX의%20위치) 5e+02)
        (Variables|Default|Set오른쪽%20%20이동인가? false))
      (else
        (CallFunction|왼쪽으로이동)
        (if (<= (Variables|Default|GetX의%20위치) 0.0)
          (Variables|Default|Set오른쪽%20%20이동인가? true))))))

(fn ConstructionScript)

(fn 오른쪽으로이동
  ;[0.15 0.15 0.15 0.5] 오른쪽으로 이동한다.
  ;;[0.15 0.15 0.15 0.5] X의 위치에 100을 더한다
  (Variables|Default|SetX의%20위치 (+ (Variables|Default|GetX의%20위치) 1e+01))
  ;;[0.15 0.15 0.15 0.5] BOX에 상대좌표 X를 "X의 위치"값으로 변경한다.
  (Transformation|SetRelativeLocation (Variables|Default|GetBox) (Math|Vector|MakeVector (Variables|Default|GetX의%20위치) 0.0 0.0) false false))

(fn 왼쪽으로이동
  ;[0.15 0.15 0.15 0.5] 왼쪽으로 이동한다.
  ;;[0.15 0.15 0.15 0.5] X의 위치에 100을 더한다
  (Variables|Default|SetX의%20위치 (+ (Variables|Default|GetX의%20위치) -1e+01))
  ;;[0.15 0.15 0.15 0.5] BOX에 상대좌표 X를 "X의 위치"값으로 변경한다.
  (Transformation|SetRelativeLocation (Variables|Default|GetBox) (Math|Vector|MakeVector (Variables|Default|GetX의%20위치) 0.0 0.0) false false))

(fn EventSwitchToggle
  (params (Toggle :type Boolean))
  (Variables|Default|Setisplay Toggle))

(fn DoPlayandStop
  (params (isplay :type Boolean))
  (Variables|Default|Setisplay isplay)
  (return true))