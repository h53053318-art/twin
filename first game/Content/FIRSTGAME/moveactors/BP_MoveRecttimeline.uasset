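; Moving actor that slides its Cube along a looping timeline path, started and stopped by a switch.
; A vector timeline, scaled by 500, drives the Cube's relative location and restarts from the beginning when finished.
; ISRIGHT selects whether starting plays the timeline forward or in reverse.
; BeginPlay binds to the Switch's update dispatcher, and several toggle functions route a boolean to DoPlay or DoStop.
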(event Custom|DoPlay
  (if (Variables|Default|GetISRIGHT)
    (bind _vector (Timeline|타임라인 Play)
      (:Update
        (Transformation|SetRelativeLocation (Variables|Default|GetCube) (* _vector 5e+02) false false))
      (:Finished
        (Timeline|타임라인 PlayFromStart)))
    (else
      (Timeline|타임라인 Reverse))))

(event Custom|DoStop
  (bind _vector (Timeline|타임라인 Stop)
    (:Update
      (Transformation|SetRelativeLocation (Variables|Default|GetCube) (* _vector 5e+02) false false))
    (:Finished
      (Timeline|타임라인 PlayFromStart))))

(event EventBeginPlay
  (EventDispatchers|BindEventtoEventDispatcherUpdateSwitch (Variables|Default|GetSwitch) (EventDispatchers|CreateEvent :!event BPMoveRecttimelineUpdateSwitch)))

(fn ConstructionScript)

(fn BPMoveRecttimelineSwitch
  (params (Toggle :type Boolean))
  (if Toggle
    (CallFunction|DoPlay)
    (else
      (CallFunction|DoStop)))
  (return))

(fn BPMoveRecttimelineUpdateSwitch
  (params (SwitchOn :type Boolean))
  (if SwitchOn
    (CallFunction|DoPlay)
    (else
      (CallFunction|DoStop))))

(fn DoPlayandStop
  (params (isplay :type Boolean))
  (if isplay
    (CallFunction|DoPlay)
    (else
      (CallFunction|DoStop)))
  (return false))