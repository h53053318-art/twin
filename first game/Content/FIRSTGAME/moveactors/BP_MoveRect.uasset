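; BP_MoveRect is an actor that moves its Cube component around a square path in the relative XZ plane.
; While Isplay is true, Tick runs a MoveType state machine cycling Right, Up, Left and Down, switching at position limits.
; Each direction function applies a fixed per-frame step without delta time, so speed depends on frame rate.
; BeginPlay binds to a Switch's update dispatcher, and several handlers can set Isplay.
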(event Custom|DoPlayAndStop_1_1
  (params (isplay :type Boolean))
  (Variables|Default|Setisplay true))

(event Custom|Dostop_1
  (Variables|Default|Setisplay false))

(event EventBeginPlay
  (EventDispatchers|BindEventtoEventDispatcherUpdateSwitch (Variables|Default|GetSwitch) (EventDispatchers|CreateEvent :!event BPMoveRectSwitchon)))

(event EventTick
  (params (DeltaSeconds :type Float%20%28single-precision%29))
  (if (Variables|Default|Getisplay)
    (switch Utilities|FlowControl|Switch|SwitchonENUM_MOVETYPE (Variables|Default|GetMoveType)
      (:NewEnumerator0
        (CallFunction|오른쪽으로이동)
        (if (>= (Variables|Default|GetX의%20위치) 5e+02)
          (Variables|Default|SetMoveType "NewEnumerator1")))
      (:NewEnumerator1
        (CallFunction|위쪽으로이동)
        (if (>= (Variables|Default|GetLocz) 5e+02)
          (Variables|Default|SetMoveType "NewEnumerator2")))
      (:NewEnumerator2
        (CallFunction|왼쪽으로이동)
        (if (<= (Variables|Default|GetX의%20위치) 0.0)
          (Variables|Default|SetMoveType "NewEnumerator3")))
      (:NewEnumerator3
        (CallFunction|아래쪽으로이동)
        (if (<= (Variables|Default|GetLocz) 0.0)
          (Variables|Default|SetMoveType "NewEnumerator0"))))))

(fn ConstructionScript)

(fn 오른쪽으로이동
  (bind _output_get (Variables|Default|SetX의%20위치 (+ (Variables|Default|GetX의%20위치) 1e+01)))
  (Transformation|SetRelativeLocation (Variables|Default|GetCube) (Math|Vector|MakeVector _output_get 0.0 (Variables|Default|GetLocz)) false false))

(fn 위쪽으로이동
  (Variables|Default|SetLocz (+ (Variables|Default|GetLocz) 1e+01))
  (Transformation|SetRelativeLocation (Variables|Default|GetCube) (Math|Vector|MakeVector (Variables|Default|GetX의%20위치) 0.0 (Variables|Default|GetLocz)) false false))

(fn 왼쪽으로이동
  (Variables|Default|SetX의%20위치 (- (Variables|Default|GetX의%20위치) 1e+01))
  (Transformation|SetRelativeLocation (Variables|Default|GetCube) (Math|Vector|MakeVector (Variables|Default|GetX의%20위치) 0.0 (Variables|Default|Getlocz)) false false))

(fn 아래쪽으로이동
  (Variables|Default|Setlocz (- (Variables|Default|Getlocz) 1e+01))
  (Transformation|SetRelativeLocation (Variables|Default|GetCube) (Math|Vector|MakeVector (Variables|Default|GetX의%20위치) 0.0 (Variables|Default|Getlocz)) false false))

(fn BPMoveRectAutoGenFunc
  (params (Toggle :type Boolean))
  (Variables|Default|Setisplay Toggle))

(fn BPMoveRectSwitchon
  (params (SwitchOn :type Boolean))
  (Variables|Default|Setisplay SwitchOn))

(fn DoPlayandStop
  (params (isplay :type Boolean))
  (Variables|Default|Setisplay isplay)
  (return true))