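; BP_updown is an actor whose static mesh moves up and down like an elevator while its play flag is on.
; Tick steps the mesh's relative Z by a fixed, frame-rate-dependent amount, reversing direction at the upper and lower limits.
; BeginPlay binds to a referenced Switch's update dispatcher, and handler functions set the play flag to start or pause motion.
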(event EventBeginPlay
  (EventDispatchers|BindEventtoEventDispatcherUpdateSwitch (Variables|Default|GetSwitch) (EventDispatchers|CreateEvent :!event BPUpdownAutoGenFunc1)))

(event EventTick
  (params (DeltaSeconds :type Float%20%28single-precision%29))
  (if (Variables|Default|Getisplay)
    (if (Variables|Default|GetIsMoveup)
      ;[0.15 0.15 0.15 0.5] 위쪽으로 이동한다
      (Variables|Default|Setlocz (+ (Variables|Default|Getlocz) 1e+01))
      (Transformation|SetRelativeLocation (Variables|Default|GetStaticMesh) (Math|Vector|MakeVector 0.0 0.0 (Variables|Default|Getlocz)) false false)
      (if (>= (Variables|Default|Getlocz) 5e+02)
        (Variables|Default|SetIsMoveup false))
      (else
        ;[0.15 0.15 0.15 0.5] 아래쪽으로 이동한다.
        (Variables|Default|Setlocz (- (Variables|Default|Getlocz) 1e+01))
        (Transformation|SetRelativeLocation (Variables|Default|GetStaticMesh) (Math|Vector|MakeVector 0.0 0.0 (Variables|Default|Getlocz)) false false)
        (if (<= (Variables|Default|Getlocz) 0.0)
          (Variables|Default|SetIsMoveup true))))))

(fn ConstructionScript)

(fn BPUpdownAutoGenFunc
  (params (Toggle :type Boolean))
  (Variables|Default|Setisplay Toggle))

(fn BPUpdownAutoGenFunc1
  (params (SwitchOn :type Boolean))
  (Variables|Default|Setisplay SwitchOn))

(fn DoPlayandStop
  (params (isplay :type Boolean))
  (Variables|Default|Setisplay isplay)
  (return true))