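; A moving actor whose Cube slides back and forth along its relative X axis, started and stopped by a linked Switch.
; A timeline scales the X offset up to 500 units, and on finishing flips ISRIGHT to alternate between Play and Reverse, forming a ping-pong loop.
; BeginPlay binds to the Switch's update dispatcher, and several boolean wrapper functions route to DoPlay or DoStop.
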(event Custom|DoPlay
  (if (Variables|Default|GetISRIGHT) :!label _label
    (bind _value (Timeline|타임라인 Play)
      (:Update
        (Transformation|SetRelativeLocation (Variables|Default|GetCube) (* _value "500.000000,0.000000,0.000000") false false))
      (:Finished
        (Variables|Default|SetISRIGHT (not (Variables|Default|GetISRIGHT)))
        (goto _label)))
    (else
      (Timeline|타임라인 Reverse))))

(event Custom|DoStop
  (bind _value (Timeline|타임라인 Stop)
    (:Update
      (Transformation|SetRelativeLocation (Variables|Default|GetCube) (* _value "500.000000,0.000000,0.000000") false false))
    (:Finished
      (Variables|Default|SetISRIGHT (not (Variables|Default|GetISRIGHT)))
      (if (Variables|Default|GetISRIGHT)
        (Timeline|타임라인 Play)
        (else
          (Timeline|타임라인 Reverse))))))

(event EventBeginPlay
  (EventDispatchers|BindEventtoEventDispatcherUpdateSwitch (Variables|Default|GetSwitch) (EventDispatchers|CreateEvent :!event BPLEFTFIGHTTIMELINESwitch)))

(fn ConstructionScript)

(fn BPLEFTFIGHTTIMELINESwitch
  (params (Toggle :type Boolean))
  (if Toggle
    (CallFunction|DoPlay)
    (else
      (CallFunction|DoStop)))
  (return))

(fn BPLEFTFIGHTTIMELINEUpdateSwitch
  (params (SwitchOn :type Boolean))
  (if SwitchOn
    (CallFunction|DoPlay)
    (else
      (CallFunction|DoStop))))

(fn DoPlayandStop
  (params (isplay :type Boolean))
  (if isplay
    (CallFunction|DoPlay)
    (else
      (CallFunction|DoStop)))
  (return false))