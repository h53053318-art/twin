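; BP_counter is an in-world counter actor that shows a number on a widget component.
; PressF increments Counter, resets it to 0 once it exceeds 9, then pushes the value to CountWidget through UpdateSetCount.
; Tick rotates the widget to face the player camera using a look-at rotation.
; ShowCount is an empty stub, with leftover text-render logic that never runs.
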(event EventBeginPlay)

(event EventPressF
  (bind _output_get (CallFunction|Countup))
  (CallFunction|Over9count0 _output_get)
  (bind _ascount_widget (Utilities|Casting|CastToCountWidget (UserInterface|GetUserWidgetObject (Variables|Default|GetWidget))))
  (Default|UpdateSetCount _ascount_widget (Variables|Default|Getcounter)))

(event EventTick
  (params (DeltaSeconds :type Float%20%28single-precision%29))
  (Transformation|SetWorldRotation (Variables|Default|GetWidget) (Math|Rotator|FindLookatRotation (Transformation|GetWorldLocation (Variables|Default|GetWidget)) (Transformation|GetActorLocation (Game|GetPlayerCameraManager 0))) false false))

(fn ConstructionScript)

(fn Countup
  ;[0.15 0.15 0.15 0.5] count를 1씩 증가
  (bind _output_get (Variables|Default|Setcounter (+ (Variables|Default|Getcounter) 1)))
  (return _output_get))

(fn Over9count0
  (params (A :type Integer))
  ;[0.15 0.15 0.15 0.5] count가  9보다 크면
  (if (> A 9)
    ;[0.15 0.15 0.15 0.5] count 0으로 변경
    (Variables|Default|Setcounter 0)))

(fn ShowCount)