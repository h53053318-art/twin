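; BP_Dummy is a damage test dummy that shows its remaining Hp on a text render component.
; The AnyDamage event passes damage to AddDemage, which subtracts it from Hp and writes the floored value to the text.
; The text updates only while the floored Hp is above -10, though Hp keeps decreasing, and the dummy has no death or reset logic.
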(event Game|Damage|EventAnyDamage
  (params (Damage :type Float%20%28single-precision%29) (DamageType :type Damage%20Type%20Object%20Reference) (InstigatedBy :type Controller%20Object%20Reference) (DamageCauser :type Actor%20Object%20Reference))
  (CallFunction|AddDemage Damage))

(fn ConstructionScript)

(fn AddDemage
  (params (Demage :type Float%20%28double-precision%29))
  (bind _output_get (Variables|Default|SetHp (- (Variables|Default|GetHp) Demage)))
  (if (> (Math|Float|Floor _output_get) -10)
    (Rendering|Components|TextRender|SetText (Variables|Default|GetTextRender) (Utilities|Text|ToText(Integer) (Math|Float|Floor _output_get)))))