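; BP_Timer is a timer that shows elapsed time as MM:SS on a TimeWidget held by its widget component.
; While Isplay is set, Tick accumulates delta time at ten times real speed and passes minutes and seconds to Showtime, which zero-pads them for display.
; A toggle handler sets Isplay, but the binding to the Switch's toggle dispatcher is disconnected, and DoPlayAndStop is an empty stub.
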(event EventBeginPlay)

(event EventTick
  (params (DeltaSeconds :type Float%20%28single-precision%29))
  (if (Variables|Default|Getisplay)
    (bind _output_get (Variables|Default|Settodeltaseconds (+ (Variables|Default|Gettodeltaseconds) (* DeltaSeconds 1e+01))))
    (CallFunction|Showtime (/ _output_get 6e+01) (Math|Float|%(Float) _output_get 6e+01))))

(fn ConstructionScript)

(fn Floattostr00
  (params (numble :type Float%20%28double-precision%29))
  (bind _returnvalue (Math|Float|Floor numble))
  (bind _returnvalue_2 (Utilities|String|ToString(Integer) _returnvalue))
  (if (< _returnvalue 10)
    (return (Utilities|String|Append "0" _returnvalue_2))
    (else
      (return _returnvalue_2))))

(fn Showtime
  (params (min :type Float%20%28double-precision%29) (sec :type Float%20%28double-precision%29))
  (bind _astime_widget (Utilities|Casting|CastToTimeWidget (UserInterface|GetUserWidgetObject (Variables|Default|GetWidget))))
  (Default|UpdateTime _astime_widget (Utilities|String|Append (CallFunction|Floattostr00 min) ":" (CallFunction|Floattostr00 sec))))

(fn BPTimerAutoGenFunc
  (params (Toggle :type Boolean))
  (Variables|Default|Setisplay Toggle))

(fn DoPlayandStop
  (params (isplay :type Boolean)))