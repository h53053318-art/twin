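; BP_Counting is a counter Blueprint that shows a single digit on a text render component.
; Each Switchtiggler event increments Count, wraps it back to zero after nine, and updates the displayed text.
; It then calls the Fclick event dispatcher so bound listeners can react to the change.
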(event EventSwitchtiggler
  (Variables|Default|SetCount (+ (Variables|Default|GetCount) 1))
  (if (> (Variables|Default|GetCount) 9)
    (Variables|Default|SetCount 0))
  (Rendering|Components|TextRender|SetText (Variables|Default|GetTextRender) (Utilities|Text|ToText(Integer) (Variables|Default|GetCount)))
  (Default|CallEventDispatcherFclick))

(fn ConstructionScript)