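; BP_LeftRight is an actor whose Cube slides back and forth along its local X axis while play is enabled.
; Tick moves it a fixed step per frame, independent of delta time, and flips direction once it passes either end of a short range.
; On BeginPlay it binds to a Switch's toggle dispatcher, which turns the motion on and off through Isplay.
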(event EventTick
  (params (DeltaSeconds :type Float%20%28single-precision%29))
  (if (Variables|Default|Getisplay)
    (if (Variables|Default|GetIsRight)
      (bind _output_get (Variables|Default|SetPosX (+ (Variables|Default|GetPosX) 1e+01)))
      (Transformation|SetRelativeLocation (Variables|Default|GetCube) (Math|Vector|MakeVector _output_get 0.0 0.0) false false)
      (if (> (Variables|Default|GetPosX) 1e+02)
        (Variables|Default|SetIsRight false))
      (else
        (bind _output_get_2 (Variables|Default|SetPosX (+ (Variables|Default|GetPosX) -1e+01)))
        (Transformation|SetRelativeLocation (Variables|Default|GetCube) (Math|Vector|MakeVector _output_get_2 0.0 0.0) false false)
        (if (< (Variables|Default|GetPosX) 0.0)
          (Variables|Default|SetIsRight true))))))

(event EventBeginPlay
  (EventDispatchers|BindEventtoEventDispatcherToggle (Variables|Default|GetSwitch) (EventDispatchers|CreateEvent :!event EventSwitchToggle)))

(fn ConstructionScript)

(fn EventSwitchToggle
  (params (Toggle :type Boolean))
  (Variables|Default|Setisplay Toggle))