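; Actor Blueprint that moves its Cube component around a rectangular loop in the local X-Z plane while switched on.
; Tick runs a MoveType state machine (right, up, left, down), stepping the relative location a fixed amount per frame and changing direction past each bound.
; BeginPlay binds to the Switch's toggle dispatcher, and EventSwitchToggle sets Isplay to start or pause the motion.
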(event EventTick
  (params (DeltaSeconds :type Float%20%28single-precision%29))
  (if (Variables|Default|Getisplay)
    (switch Utilities|FlowControl|Switch|SwitchonEN_MoveType (Variables|Default|GetMoveType)
      (:NewEnumerator0
        (bind _output_get (Variables|Default|SetPosX (+ (Variables|Default|GetPosX) 1e+01)))
        (Transformation|SetRelativeLocation (Variables|Default|GetCube) (Math|Vector|MakeVector _output_get 0.0 (Variables|Default|GetPosZ)) false false)
        (if (> (Variables|Default|GetPosX) 1e+02)
          (Variables|Default|SetMoveType "NewEnumerator1")))
      (:NewEnumerator1
        (bind _output_get_2 (Variables|Default|SetPosZ (+ (Variables|Default|GetPosZ) 1e+01)))
        (Transformation|SetRelativeLocation (Variables|Default|GetCube) (Math|Vector|MakeVector (Variables|Default|GetPosX) 0.0 _output_get_2) false false)
        (if (> (Variables|Default|GetPosZ) 1e+02)
          (Variables|Default|SetMoveType "NewEnumerator2")))
      (:NewEnumerator2
        (bind _output_get_3 (Variables|Default|SetPosX (+ (Variables|Default|GetPosX) -1e+01)))
        (Transformation|SetRelativeLocation (Variables|Default|GetCube) (Math|Vector|MakeVector _output_get_3 0.0 (Variables|Default|GetPosZ)) false false)
        (if (< (Variables|Default|GetPosX) 0.0)
          (Variables|Default|SetMoveType "NewEnumerator3")))
      (:NewEnumerator3
        (bind _output_get_4 (Variables|Default|SetPosZ (+ (Variables|Default|GetPosZ) -1e+01)))
        (Transformation|SetRelativeLocation (Variables|Default|GetCube) (Math|Vector|MakeVector (Variables|Default|GetPosX) 0.0 _output_get_4) false false)
        (if (< (Variables|Default|GetPosZ) 0.0)
          (Variables|Default|SetMoveType "NewEnumerator0"))))))

(event EventBeginPlay
  (EventDispatchers|BindEventtoEventDispatcherToggle (Variables|Default|GetSwitch) (EventDispatchers|CreateEvent :!event EventSwitchToggle)))

(fn ConstructionScript)

(fn EventSwitchToggle
  (params (Toggle :type Boolean))
  (Variables|Default|Setisplay Toggle))