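; BP_Timer1 is a timer that shows elapsed time as minutes:seconds on a TextRender, counting at ten times real speed.
; BeginPlay binds to the referenced Switch's event dispatcher, and the switch handler sets Isplay from its toggle.
; While Isplay is true, Tick accumulates scaled delta time and passes it to Showtime.
; FloatToStr00 floors each value and zero-pads only those below 9.
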(event EventTick
  (params (DeltaSeconds :type Float%20%28single-precision%29))
  (if (Variables|Default|Getisplay)
    (bind _output_get (Variables|Default|SetTotaldeltaseconds (+ (* DeltaSeconds 1e+01) (Variables|Default|GetTotaldeltaseconds))))
    (CallFunction|Showtime (/ _output_get 6e+01) (Math|Float|%(Float) _output_get 6e+01))))

(event EventBeginPlay
  (EventDispatchers|BindEventtoEventDispatcherSwitch (Variables|Default|GetSwitch) (EventDispatchers|CreateEvent :!event BPTimer1Switch)))

(fn ConstructionScript)

(fn FloattoStr00
  (params (numble :type Float%20%28double-precision%29))
  (bind _returnvalue (Math|Float|Floor numble))
  (bind _returnvalue_2 (Utilities|String|ToString(Integer) _returnvalue))
  (if (< _returnvalue 9.0)
    (return (Utilities|String|Append "0" _returnvalue_2))
    (else
      (return _returnvalue_2))))

(fn Showtime
  (params (min :type Float%20%28double-precision%29) (sec :type Float%20%28double-precision%29))
  (Rendering|Components|TextRender|SetText (Variables|Default|GetTextRender) (Utilities|Text|ToText(String) (Utilities|String|Append (CallFunction|FloattoStr00 min) ":" (CallFunction|FloattoStr00 sec)))))

(fn BPTimer1Switch
  (params (toggle :type Boolean))
  (Variables|Default|Setisplay toggle))