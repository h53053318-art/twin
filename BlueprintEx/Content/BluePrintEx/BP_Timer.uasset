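; BP_Timer is an actor that displays a running minutes:seconds clock on a TextRender component.
; BeginPlay binds to a Switch's toggle dispatcher, with EventSwitchToggle setting the Isplay flag that gates counting.
; While active, Tick accumulates delta time at ten times real speed, and ShowTime renders it through a zero-padding helper.
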(event EventTick
  (params (DeltaSeconds :type Float%20%28single-precision%29))
  (if (Variables|Default|Getisplay)
    (bind _output_get (Variables|Default|SetTotaldeltaseconds (+ (* DeltaSeconds 1e+01) (Variables|Default|GetTotaldeltaseconds))))
    (CallFunction|ShowTime (/ _output_get 6e+01) (Math|Float|%(Float) _output_get 6e+01))))

(event EventBeginPlay
  (EventDispatchers|BindEventtoEventDispatcherToggle (Variables|Default|GetSwitch) (EventDispatchers|CreateEvent :!event EventSwitchToggle)))

(fn ConstructionScript)

(fn FloattoStr00
  (params (number :type Float%20%28double-precision%29))
  (bind _returnvalue (Math|Float|Floor number))
  (bind _returnvalue_2 (Utilities|String|ToString(Integer) _returnvalue))
  (if (< number 1e+01)
    (return (Utilities|String|Append "0" _returnvalue_2))
    (else
      (return _returnvalue_2))))

(fn ShowTime
  (params (min :type Float%20%28double-precision%29) (sec :type Float%20%28double-precision%29))
  (Rendering|Components|TextRender|SetText (Variables|Default|GetTextRender) (Utilities|Text|ToText(String) (Utilities|String|Append (CallFunction|FloattoStr00 min) ":" (CallFunction|FloattoStr00 sec)))))

(fn EventSwitchToggle
  (params (Toggle :type Boolean))
  (Variables|Default|Setisplay Toggle))