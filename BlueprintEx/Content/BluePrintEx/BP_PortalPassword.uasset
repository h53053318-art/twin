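; BP_PortalPassword is a password puzzle that shows a Sphere when a set of count boxes displays the correct code.
; On BeginPlay it hides the Sphere and binds to the click dispatcher of each box in the Counts array.
; The press-F function sets the Sphere's visibility from Isallbox9, which compares each box's Count to the Password entry at the same index and fails on the first mismatch.
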(event EventBeginPlay
  (Rendering|SetVisibility (Variables|Default|GetSphere) false false)
  ;[0.15 0.15 0.15 0.5] count박스 이벤트 바인딩
  (for _array_element (Variables|Default|Getcounts)
    (EventDispatchers|BindEventtoEventDispatcherFclick _array_element (EventDispatchers|CreateEvent :!event BPPortalPressF))))

(fn ConstructionScript)

(fn BPPortalPressF
  (Rendering|SetVisibility (Variables|Default|GetSphere) (CallFunction|Isallbox9) false))

(fn Isallbox9
  (for (_array_element _array_index) (Variables|Default|Getcounts)
    (if (not (== (Variables|/Game/BluePrintEx/BP_Counting.BP_Counting_C|GetCount _array_element) (Utilities|Array|Get(acopy) (Variables|Default|GetPassword) _array_index)))
      (return false)))
  (return true))