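; Test actor that moves its Cube component around a square loop in the local XZ plane while Isplay is true.
; Each Tick, a switch on MOVETYPE steps the tracked X or Z position by a fixed amount, applies it as relative location, and advances the state at each corner.
; Steps ignore delta time, so speed depends on frame rate.
; Despite their names, DOWN moves along -X and LEFT along -Z.
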(event EventTick
  (params (DeltaSeconds :type Float%20%28single-precision%29))
  (if (Variables|Default|Getisplay)
    (switch Utilities|FlowControl|Switch|SwitchonENUM_TYPE (Variables|Default|GetMOVETYPE)
      (:NewEnumerator0
        (bind _output_get (Variables|Default|Setx의%20위치 (+ (Variables|Default|Getx의%20위치) 1e+01)))
        (Transformation|SetRelativeLocation (Variables|Default|GetCube) (Math|Vector|MakeVector _output_get 0.0 0.0) false false)
        (if (>= (Variables|Default|Getx의%20위치) 5e+02)
          (Variables|Default|SetMOVETYPE "NewEnumerator1")))
      (:NewEnumerator1
        (bind _output_get_2 (Variables|Default|SetZ의%20위치 (+ (Variables|Default|GetZ의%20위치) 1e+01)))
        (Transformation|SetRelativeLocation (Variables|Default|GetCube) (Math|Vector|MakeVector (Variables|Default|Getx의%20위치) 0.0 _output_get_2) false false)
        (if (>= (Variables|Default|GetZ의%20위치) 5e+02)
          (Variables|Default|SetMOVETYPE "NewEnumerator2")))
      (:NewEnumerator2
        (bind _output_get_3 (Variables|Default|Setx의%20위치 (+ (Variables|Default|Getx의%20위치) -1e+01)))
        (Transformation|SetRelativeLocation (Variables|Default|GetCube) (Math|Vector|MakeVector _output_get_3 0.0 (Variables|Default|GetZ의%20위치)) false false)
        (if (<= (Variables|Default|Getx의%20위치) 0.0)
          (Variables|Default|SetMOVETYPE "NewEnumerator3")))
      (:NewEnumerator3
        (bind _output_get_4 (Variables|Default|SetZ의%20위치 (+ (Variables|Default|GetZ의%20위치) -1e+01)))
        (Transformation|SetRelativeLocation (Variables|Default|GetCube) (Math|Vector|MakeVector (Variables|Default|Getx의%20위치) 0.0 _output_get_4) false false)
        (if (<= (Variables|Default|GetZ의%20위치) 0.0)
          (Variables|Default|SetMOVETYPE "NewEnumerator0"))))))

(fn ConstructionScript)