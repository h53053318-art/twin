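; BP_LeftRight is a test Blueprint that slides its Cube component back and forth along the relative X axis.
; While Isplay is true, each Tick adds a fixed step to the stored X position (X의위치) and applies it with SetRelativeLocation.
; Isright sets the direction and flips at fixed upper and lower limits.
; The step ignores delta time, so speed depends on frame rate.
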(event EventTick
  (params (DeltaSeconds :type Float%20%28single-precision%29))
  (if (Variables|Default|Getisplay)
    (if (Variables|Default|Getisright)
      (bind _output_get (Variables|Default|Setx의%20위치 (+ (Variables|Default|Getx의%20위치) 1e+01)))
      (Transformation|SetRelativeLocation (Variables|Default|GetCube) (Math|Vector|MakeVector _output_get 0.0 0.0) false false)
      (if (>= (Variables|Default|Getx의%20위치) 5e+02)
        (Variables|Default|Setisright false))
      (else
        (bind _output_get_2 (Variables|Default|Setx의%20위치 (+ (Variables|Default|Getx의%20위치) -1e+01)))
        (Transformation|SetRelativeLocation (Variables|Default|GetCube) (Math|Vector|MakeVector _output_get_2 0.0 0.0) false false)
        (if (<= (Variables|Default|Getx의%20위치) 0.0)
          (Variables|Default|Setisright true))))))

(fn ConstructionScript)