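; BP_Switch is a test switch that starts and stops a set of actors in the Actors array.
; Its PressF event flips a toggle, casts each actor to BP_playstop and passes the new state to DoPlayandStop.
; Unused Move and Stop functions use cast chains to drive BP_LeftRight, BP_LeftRightTime, BP_Rect or BP_Timer directly.
; The Cube overlap events are empty.
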(event OnComponentBeginOverlap(Cube)
  (params (OverlappedComponent :type Primitive%20Component%20Object%20Reference) (OtherActor :type Actor%20Object%20Reference) (OtherComp :type Primitive%20Component%20Object%20Reference) (OtherBodyIndex :type Integer) (bFromSweep :type Boolean) (SweepResult :type Hit%20Result%20Structure%20%28by%20ref%29)))

(event OnComponentEndOverlap(Cube)
  (params (OverlappedComponent :type Primitive%20Component%20Object%20Reference) (OtherActor :type Actor%20Object%20Reference) (OtherComp :type Primitive%20Component%20Object%20Reference) (OtherBodyIndex :type Integer)))

(event EventPressF
  (bind _output_get (Variables|Default|SetToggle (not (Variables|Default|GetToggle))))
  (if _output_get
    (for _array_element (Variables|Default|Getactors)
      (bind _asbp_playstop (Utilities|Casting|CastToBP_playstop _array_element))
      (Default|DoPlayandStop _asbp_playstop true))
    (else
      (for _array_element_2 (Variables|Default|Getactors)
        (bind _asbp_playstop_2 (Utilities|Casting|CastToBP_playstop _array_element_2))
        (Default|DoPlayandStop _asbp_playstop_2 false)))))

(fn ConstructionScript)

(fn Move
  (params (Object :type Object%20Object%20Reference) (Object2 :type Object%20Object%20Reference) (Object3 :type Object%20Object%20Reference) (Object4 :type Object%20Object%20Reference))
  (bind _asbp_left_right (Utilities|Casting|CastToBP_LeftRight Object4)
    (:then
      (Variables|/Game/test/Moverect/BP_LeftRight.BP_LeftRight_C|Setisplay _asbp_left_right true))
    (:CastFailed
      (bind _asbp_left_right_time (Utilities|Casting|CastToBP_LeftRightTime Object)
        (:then
          (Default|DoPlay _asbp_left_right_time))
        (:CastFailed
          (bind _asbp_rect (Utilities|Casting|CastToBP_Rect Object2)
            (:then
              (Variables|/Game/test/Moverect/BP_Rect.BP_Rect_C|Setisplay _asbp_rect true))
            (:CastFailed
              (bind _asbp_timer (Utilities|Casting|CastToBP_Timer Object3))
              (Variables|/Game/test/BP_Timer.BP_Timer_C|Setisplay _asbp_timer true))))))))

(fn Stop
  (params (Object :type Object%20Object%20Reference) (Object2 :type Object%20Object%20Reference) (Object3 :type Object%20Object%20Reference) (Object4 :type Object%20Object%20Reference))
  (bind _asbp_left_right (Utilities|Casting|CastToBP_LeftRight Object4)
    (:then
      (Variables|/Game/test/Moverect/BP_LeftRight.BP_LeftRight_C|Setisplay _asbp_left_right false))
    (:CastFailed
      (bind _asbp_left_right_time (Utilities|Casting|CastToBP_LeftRightTime Object)
        (:then
          (Default|DoStop _asbp_left_right_time))
        (:CastFailed
          (bind _asbp_rect (Utilities|Casting|CastToBP_Rect Object2)
            (:then
              (Variables|/Game/test/Moverect/BP_Rect.BP_Rect_C|Setisplay _asbp_rect false))
            (:CastFailed
              (bind _asbp_timer (Utilities|Casting|CastToBP_Timer Object3))
              (Variables|/Game/test/BP_Timer.BP_Timer_C|Setisplay _asbp_timer false))))))))