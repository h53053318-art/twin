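; BP_Timer is a count-up timer that shows minutes and seconds on a TextRender component.
; While Isplay is set, Tick accumulates delta time at ten times real speed and passes derived minutes and seconds to Showtime.
; Showtime uses Floatstr00 to floor and zero-pad each value, then joins them with a colon.
; DoPlayandStop sets Isplay to start or pause counting, without resetting the total.
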(event EventTick
  (params (DeltaSeconds :type Float%20%28single-precision%29))
  (if (Variables|Default|Getisplay)
    (bind _output_get (Variables|Default|Settodeltasecs (+ (Variables|Default|Gettodeltasecs) (* DeltaSeconds 1e+01))))
    (CallFunction|Showtime (/ _output_get 6e+01) (Math|Float|%(Float) _output_get 6e+01))))

(fn ConstructionScript)

(fn Floatstr00
  (params (numble :type Float%20%28double-precision%29))
  (bind _returnvalue (Math|Float|Floor numble))
  (bind _returnvalue_2 (Utilities|String|ToString(Integer) _returnvalue))
  (if (< _returnvalue 10)
    (return (Utilities|String|Append "0" _returnvalue_2))
    (else
      (return _returnvalue_2))))

(fn Showtime
  (params (min :type Float%20%28double-precision%29) (secs :type Float%20%28double-precision%29))
  (Rendering|Components|TextRender|SetText (Variables|Default|GetTextRender) (|GenerictoText (Utilities|String|Append (CallFunction|Floatstr00 min) ":" (CallFunction|Floatstr00 secs)))))

(fn DoPlayandStop
  (params (isplay :type Boolean))
  (Variables|Default|Setisplay isplay)
  (return false))