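; BP_Timer1 is a test timer that displays a running minutes:seconds count on a TextRender component.
; Tick accumulates delta time at ten times real speed, splits it into minutes and seconds, and passes them to Showtime.
; Showtime joins two formatting helpers with a colon: Floatstr00 zero-pads seconds below ten, while NewFunction always prefixes minutes with a zero, as both of its branches give the same result.
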(event EventTick
  (params (DeltaSeconds :type Float%20%28single-precision%29))
  (if true
    (bind _output_get (Variables|Default|SetTodelasecs (+ (Variables|Default|GetTodelasecs) (* DeltaSeconds 1e+01))))
    (CallFunction|Showtime (/ _output_get 6e+01) (Math|Float|%(Float) _output_get 6e+01))))

(fn ConstructionScript)

(fn Floatstr00
  (params (number :type Float%20%28double-precision%29))
  (bind _returnvalue (Math|Float|Floor number))
  (bind _returnvalue_2 (Utilities|String|ToString(Integer) _returnvalue))
  (if (< _returnvalue 10)
    (return (Utilities|String|Append "0" _returnvalue_2))
    (else
      (return _returnvalue_2))))

(fn NewFunction
  (params (A :type Float%20%28double-precision%29))
  (bind _returnvalue (Math|Float|Floor A))
  (if (< _returnvalue 10)
    _
    (else
      _))
  (return (Utilities|String|Append "0" (Utilities|String|ToString(Integer) _returnvalue))))

(fn Showtime
  (params (min :type Float%20%28double-precision%29) (secs :type Float%20%28double-precision%29))
  (Rendering|Components|TextRender|SetText (Variables|Default|GetTextRender) (|GenerictoText (Utilities|String|Append (CallFunction|NewFunction min) ":" (CallFunction|Floatstr00 secs)))))