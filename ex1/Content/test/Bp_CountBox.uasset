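; Bp_CountBox is a test Blueprint that shows a single-digit counter on a TextRender component.
; Pressing F increments Count, wraps it back to zero once it passes nine, and writes the new value to the text.
; The construction script is empty, and a stray sequence node in the event graph is never executed.
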(event EventPressF
  (Variables|Default|Setcount (+ (Variables|Default|Getcount) 1))
  (if (> (Variables|Default|Getcount) 9)
    (Variables|Default|Setcount 0))
  (Rendering|Components|TextRender|SetText (Variables|Default|GetTextRender) (Utilities|Text|ToText(Integer) (Variables|Default|Getcount))))

(fn ConstructionScript)