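; BP_Portal1 is a level-exit portal that opens Lv1_ThirdPerson when its sphere is overlapped.
; It hides the sphere at BeginPlay and binds to each BP_Coin1's Getcoin dispatcher.
; ShowPor reveals the sphere when RemainCoin counts no coins left.
; Only visibility is toggled, and the overlap event loads the level without checking the coin count.
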(event OnComponentBeginOverlap(Sphere)
  (params (OverlappedComponent :type Primitive%20Component%20Object%20Reference) (OtherActor :type Actor%20Object%20Reference) (OtherComp :type Primitive%20Component%20Object%20Reference) (OtherBodyIndex :type Integer) (bFromSweep :type Boolean) (SweepResult :type Hit%20Result%20Structure%20%28by%20ref%29))
  (Game|OpenLevel(byName) "Lv1_ThirdPerson"))

(event EventBeginPlay
  (Rendering|SetVisibility (Variables|Default|GetSphere) false false)
  (bind _outactors (Actor|GetAllActorsOfClass "/Game/EX/BP_Coin1.BP_Coin1_C"))
  (for _array_element _outactors
    (EventDispatchers|BindEventtoEventDispatcherGetcoin _array_element (EventDispatchers|CreateEvent :!event ShowPor))))

(fn ConstructionScript)

(fn ShowPor
  (Rendering|SetVisibility (Variables|Default|GetSphere) (== (CallFunction|RemainCoin) 0) false))

(fn RemainCoin
  (bind _outactors (Actor|GetAllActorsOfClass "/Game/EX/BP_Coin1.BP_Coin1_C"))
  (for _array_element _outactors
    (if (not (Game|IsActorBeingDestroyed))
      (LocalVariables|Setcoin (+ (LocalVariables|Getcoin) 1))))
  (return (LocalVariables|Getcoin)))