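; BP_Coin1 is a collectible coin that the player picks up by touching it.
; Tick spins the Sphere component by a fixed step each frame, independent of delta time.
; When a player-controlled Character overlaps Sphere1, the coin calls GetCoin on that player's BP_Hud1.
; It then destroys itself and fires its Getcoin event dispatcher after the destroy call.
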(event OnComponentBeginOverlap(Sphere1)
  (params (OverlappedComponent :type Primitive%20Component%20Object%20Reference) (OtherActor :type Actor%20Object%20Reference) (OtherComp :type Primitive%20Component%20Object%20Reference) (OtherBodyIndex :type Integer) (bFromSweep :type Boolean) (SweepResult :type Hit%20Result%20Structure%20%28by%20ref%29))
  (bind _as캐릭터 (Utilities|Casting|CastToCharacter OtherActor))
  (bind _as플레이어_컨트롤러 (Utilities|Casting|CastToPlayerController (Pawn|GetController _as캐릭터)))
  (bind _asbp_hud_1 (Utilities|Casting|CastToBP_Hud1 (HUD|GetHUD _as플레이어_컨트롤러)))
  (Default|GetCoin _asbp_hud_1)
  (Actor|DestroyActor)
  (Default|CallEventDispatcherGetcoin))

(event EventTick
  (params (DeltaSeconds :type Float%20%28single-precision%29))
  (Transformation|AddRelativeRotation (Variables|Default|GetSphere) "0.000000,5.000000,0.000000" false false))

(fn ConstructionScript)