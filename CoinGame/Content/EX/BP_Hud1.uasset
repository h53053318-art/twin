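; BP_Hud1 is a HUD Blueprint that shows how many BP_Coin1 pickups remain in the level.
; On BeginPlay it creates the HudWidGet1 widget, binds to every coin's Getcoin dispatcher and calls GetCoin for the initial display.
; GetCoin passes the result of RemainCoin to the widget's Showcoin.
; RemainCoin recounts coin actors, skipping any being destroyed so a just-collected coin is excluded.
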(event EventBeginPlay
  (bind _returnvalue (UserInterface|CreateWidget "/Game/EX/HudWidGet1.HudWidGet1_C"))
  (bind _output_get (Variables|Default|SetHudwidget1 _returnvalue))
  (UserInterface|Viewport|AddtoViewport _output_get 0)
  (bind _outactors (Actor|GetAllActorsOfClass "/Game/EX/BP_Coin1.BP_Coin1_C"))
  (for _array_element _outactors
    (EventDispatchers|BindEventtoEventDispatcherGetcoin _array_element (EventDispatchers|CreateEvent :!event GetCoin)))
  (CallFunction|GetCoin))

(fn ConstructionScript)

(fn GetCoin
  (Default|Showcoin (Variables|Default|GetHudwidget1) (CallFunction|RemainCoin)))

(fn RemainCoin
  (bind _outactors (Actor|GetAllActorsOfClass "/Game/EX/BP_Coin1.BP_Coin1_C"))
  (for _array_element _outactors
    (if (not (Game|IsActorBeingDestroyed _array_element))
      (LocalVariables|Setcoin (+ (LocalVariables|Getcoin) 1))))
  (return (LocalVariables|Getcoin)))